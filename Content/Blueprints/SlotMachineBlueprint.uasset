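; Slot machine Blueprint that positions a pointer component to indicate the current value.
; Every Tick moves the Pointer to a fixed forward offset at the stored height, then recalculates that height for the next frame.
; SetPointerHeight converts CurrentValue linearly into a vertical position, stepping the pointer down at even intervals as the value rises.
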(event EventTick
  (params (DeltaSeconds :type Float%20%28single-precision%29))
  (Transformation|SetRelativeLocation (Variables|Default|GetPointer) (Math|Vector|MakeVector 1.3e+02 0.0 (Variables|Default|GetPointerHeight)) false)
  (CallFunction|SetPointerHeight))

(fn ConstructionScript)

(fn SetPointerHeight
  (Variables|Default|SetPointerHeight (- 168.0 (Math|Conversions|ToFloat(Integer) (* (- (Variables|Default|GetcurrentValue) 1) 68)))))