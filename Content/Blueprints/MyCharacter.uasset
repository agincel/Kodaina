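; Player character for a dice-driven board game with turn-based battles, run by a turn-state machine.
; A looping timer cycles the die until stopped; timelines then slide the character between overlapped Space actors, with a direction history refunding backtracked steps.
; Confirming a space heals or opens the battle HUD, where the action button cycles moves and hit events apply defense-reduced damage.
; Directional flipbook switching is unfinished and disconnected.
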(event Custom|UpdateAnimation
  ;[1 1 1] Calling Animation Switcher and Switching the Flipbook
)

(event EventBeginPlay
  ;[1 1 1] Begin Play
  (bind _returnvalue (UserInterface|CreateWidget "/Game/Blueprints/RollingMovingHUD.RollingMovingHUD_C"))
  (UserInterface|Viewport|AddtoViewport _returnvalue)
  (Variables|Default|SetRollingHUD _returnvalue))

(event EventPhysicalAttackHit
  (params (Enemy%20Attack :type Float%20%28single-precision%29))
  ;[1 1 1] Physical Attack Hit
  (if (<= (- (Variables|Default|GetCurrent%20HP) (- Enemy%20Attack (/ (Variables|Default|GetBaseDefense) 1.75))) 0.0)
    (Variables|Default|SetCurrent%20HP 0.0)
    (else
      (Variables|Default|SetCurrent%20HP (- (Variables|Default|GetCurrent%20HP) (- Enemy%20Attack (/ (Variables|Default|GetBaseDefense) 1.75)))))))

(event EventMagicAttackHit
  (params (Enemy%20Attack :type Float%20%28single-precision%29))
  ;[1 1 1] Magic Attack Hit
  (if (<= (- (Variables|Default|GetCurrent%20HP) (- Enemy%20Attack (/ (Variables|Default|GetBaseMagicDefense) 1.75))) 0.0)
    (Variables|Default|SetCurrent%20HP 0.0)
    (else
      (Variables|Default|SetCurrent%20HP (- (Variables|Default|GetCurrent%20HP) (- Enemy%20Attack (/ (Variables|Default|GetBaseMagicDefense) 1.75)))))))

(event EventSetMove
  (params (ToState :type BattleMoveState%20Enum :default "NewEnumerator4"))
  (Variables|Default|SetBattleMoves ToState))

(event Input|ActionEvents|InputActionActionButton
  ;[1 1 1] Space Pressed
  (:Pressed
    (switch Utilities|FlowControl|Switch|SwitchonTurnState (Variables|Default|GetCurrentTurnState)
      (:NewEnumerator5
        (if (Variables|Default|GetStateIsTurn) :!label _label
          (if (Utilities|Enum|Equal(Enum) (Variables|Default|GetCurrentTurnState) "NewEnumerator5")
            (if (== 0 (Variables|Default|GetdiceRoll))
              (Utilities|Time|SetTimerbyFunctionName 0 "RollTheDice" 0.07 true)
              (Utilities|Array|Clear (Variables|Default|GetmovementArray))
              (Variables|Default|SethasMoved false)
              (Variables|Default|SetCurrentTurnState "NewEnumerator1"))
            (else
              (Utilities|Time|ClearTimerbyFunctionName 0 "RollTheDice")
              (Variables|Default|SetCurrentTurnState "NewEnumerator0")))))
      (:NewEnumerator1
        (goto _label))
      (:NewEnumerator0
        (goto _label))
      (:NewEnumerator3
        (switch Utilities|FlowControl|Switch|SwitchonBattleMoveState (Variables|Default|GetBattleMoves)
          (:NewEnumerator4
            (Variables|Default|SetBattleMoves "NewEnumerator0"))
          (:NewEnumerator0
            (Variables|Default|SetBattleMoves "NewEnumerator1"))
          (:NewEnumerator1
            (Variables|Default|SetBattleMoves "NewEnumerator5"))
          (:NewEnumerator5
            (Variables|Default|SetBattleMoves "NewEnumerator2"))
          (:NewEnumerator2
            (Variables|Default|SetBattleMoves "NewEnumerator4")))))))

(event Input|ActionEvents|InputActionBattleStepper
  ;[1 1 1] Enter Pressed
  (:Pressed
    (switch Utilities|FlowControl|Switch|SwitchonTurnState (Variables|Default|GetCurrentTurnState)
      (:NewEnumerator5
        (if (Variables|Default|GethasMoved)
          (bind _type (CallFunction|GetOccupiedSpaceType))
          (switch Utilities|FlowControl|Switch|SwitchonSpaceTypes _type
            (:NewEnumerator0
              (Widget|RemovefromParent (Variables|Default|GetRollingHUD))
              (bind _returnvalue (UserInterface|CreateWidget "/Game/Blueprints/BattleHUD.BattleHUD_C"))
              (UserInterface|Viewport|AddtoViewport _returnvalue)
              (Variables|Default|SetBattleHUD _returnvalue)
              (Variables|Default|SetCurrentTurnState "NewEnumerator3"))
            (:NewEnumerator1
              (Variables|Default|SetCurrent%20HP (Variables|Default|GetMax%20HP))
              (Variables|Default|SethasMoved false)
              (Utilities|Array|Clear (Variables|Default|GetmovementArray))))))
      (:NewEnumerator3
        (Default|BeginBattle (Variables|Default|GetBattleHUD))))))

(event Input|AxisEvents|InputAxisMoveRight
  (params (AxisValue :type Float%20%28single-precision%29))
  ;[1 1 1] Input Right
  (switch Utilities|FlowControl|Switch|SwitchonTurnState (Variables|Default|GetCurrentTurnState)
    (:NewEnumerator5
      _)
    (:NewEnumerator0
      _))
  (if (Variables|Default|GetStateIsTurn)
    (Math|Float|CompareFloat AxisValue 0.0
      (:>
        (Variables|Default|SetisIdleLeft false)
        (Variables|Default|SetisIdleRight true)
        (Variables|Default|SetisIdleUp false)
        (Variables|Default|SetisIdleDown false)
        (if (not (Utilities|Enum|Equal(Enum) (Variables|Default|GetCurrentTurnState) "NewEnumerator1"))
          (bind _outputspace (CallFunction|MoveSpace (Variables|Default|GetCollisionRight) false "r"))
          (if (Variables|Default|GetvalidMove)
            (bind _alpha (Timeline|Timeline_0 PlayFromStart)
              (:Update
                (CallFunction|UpdateAnimation)
                (Transformation|SetActorLocation (Math|Vector|Lerp(Vector) (Transformation|GetActorLocation) (Transformation|GetActorLocation _outputspace) _alpha) false)
                (Variables|Default|SetBoardSpot (Math|Vector|Lerp(Vector) (Transformation|GetActorLocation) (Transformation|GetActorLocation _outputspace) _alpha))
                (Variables|Default|SetcanMoveUpDown false)
                (Variables|Default|SetcanMoveLeftRight false)
                (Variables|Default|SetvalidMove false))))))
      (:==
        (Variables|Default|SetcanMoveLeftRight true))
      (:<
        (Variables|Default|SetisIdleLeft true)
        (Variables|Default|SetisIdleRight false)
        (Variables|Default|SetisIdleUp false)
        (Variables|Default|SetisIdleDown false)
        (if (not (Utilities|Enum|Equal(Enum) (Variables|Default|GetCurrentTurnState) "NewEnumerator1"))
          (bind _outputspace_2 (CallFunction|MoveSpace (Variables|Default|GetCollisionLeft) false "l"))
          (if (Variables|Default|GetvalidMove)
            (bind _alpha_2 (Timeline|Timeline1 PlayFromStart)
              (:Update
                (CallFunction|UpdateAnimation)
                (Transformation|SetActorLocation (Math|Vector|Lerp(Vector) (Transformation|GetActorLocation) (Transformation|GetActorLocation _outputspace_2) _alpha_2) false)
                (Variables|Default|SetBoardSpot (Math|Vector|Lerp(Vector) (Transformation|GetActorLocation) (Transformation|GetActorLocation _outputspace_2) _alpha_2))
                (Variables|Default|SetcanMoveUpDown false)
                (Variables|Default|SetcanMoveLeftRight false)
                (Variables|Default|SetvalidMove false)))))))))

(event Input|AxisEvents|InputAxisMoveUp
  (params (AxisValue :type Float%20%28single-precision%29))
  ;[1 1 1] Input Up
  (switch Utilities|FlowControl|Switch|SwitchonTurnState (Variables|Default|GetCurrentTurnState)
    (:NewEnumerator5
      _)
    (:NewEnumerator0
      _))
  (if (Variables|Default|GetStateIsTurn)
    (Math|Float|CompareFloat AxisValue 0.0
      (:>
        (Variables|Default|SetisIdleLeft false)
        (Variables|Default|SetisIdleRight false)
        (Variables|Default|SetisIdleUp true)
        (Variables|Default|SetisIdleDown false)
        (if (not (Utilities|Enum|Equal(Enum) (Variables|Default|GetCurrentTurnState) "NewEnumerator1"))
          (bind _outputspace (CallFunction|MoveSpace (Variables|Default|GetCollisionUp) true "u"))
          (if (Variables|Default|GetvalidMove)
            (bind _alpha (Timeline|Timeline2 PlayFromStart)
              (:Update
                (CallFunction|UpdateAnimation)
                (Transformation|SetActorLocation (Math|Vector|Lerp(Vector) (Transformation|GetActorLocation) (Transformation|GetActorLocation _outputspace) _alpha) false)
                (Variables|Default|SetBoardSpot (Math|Vector|Lerp(Vector) (Transformation|GetActorLocation) (Transformation|GetActorLocation _outputspace) _alpha))
                (Variables|Default|SetcanMoveUpDown false)
                (Variables|Default|SetcanMoveLeftRight false)
                (Variables|Default|SetvalidMove false))))))
      (:==
        (Variables|Default|SetcanMoveUpDown true))
      (:<
        (Variables|Default|SetisIdleLeft false)
        (Variables|Default|SetisIdleRight false)
        (Variables|Default|SetisIdleUp false)
        (Variables|Default|SetisIdleDown true)
        (if (not (Utilities|Enum|Equal(Enum) (Variables|Default|GetCurrentTurnState) "NewEnumerator1"))
          (bind _outputspace_2 (CallFunction|MoveSpace (Variables|Default|GetCollisionDown) true "d"))
          (if (Variables|Default|GetvalidMove)
            (bind _alpha_2 (Timeline|Timeline3 PlayFromStart)
              (:Update
                (CallFunction|UpdateAnimation)
                (Transformation|SetActorLocation (Math|Vector|Lerp(Vector) (Transformation|GetActorLocation) (Transformation|GetActorLocation _outputspace_2) _alpha_2) false)
                (Variables|Default|SetBoardSpot (Math|Vector|Lerp(Vector) (Transformation|GetActorLocation) (Transformation|GetActorLocation _outputspace_2) _alpha_2))
                (Variables|Default|SetcanMoveUpDown false)
                (Variables|Default|SetcanMoveLeftRight false)
                (Variables|Default|SetvalidMove false)))))))))

(fn ConstructionScript)

(fn AnimationSwitcher
  (params (isFacingLeft :type Boolean) (isFacingRight :type Boolean) (isFacingUp :type Boolean) (isFacingDown :type Boolean) (Velocity :type Vector))
  (bind (_x _y _z) (Math|Vector|BreakVector Velocity))
  ;[1 1 1] Animation State Machine
  (LocalVariables|Setx_vel _x)
  (LocalVariables|Setz_vel _z)
  (if isFacingLeft
    (if (> 0.0 (LocalVariables|Getx_vel))
      (LocalVariables|SetAnimationState "NewEnumerator4")
      (else
        (LocalVariables|SetAnimationState "NewEnumerator0")))
    (return (Utilities|Select :Index (LocalVariables|GetAnimationState) :NewEnumerator0 0 :NewEnumerator1 0 :NewEnumerator2 0 :NewEnumerator3 0 :NewEnumerator4 0 :NewEnumerator5 0 :NewEnumerator6 0 :NewEnumerator7 0))
    (elif isFacingRight
      (if (> (LocalVariables|Getx_vel) 0.0)
        (LocalVariables|SetAnimationState "NewEnumerator5")
        (else
          (LocalVariables|SetAnimationState "NewEnumerator1")))
      (return (Utilities|Select :Index (LocalVariables|GetAnimationState) :NewEnumerator0 0 :NewEnumerator1 0 :NewEnumerator2 0 :NewEnumerator3 0 :NewEnumerator4 0 :NewEnumerator5 0 :NewEnumerator6 0 :NewEnumerator7 0))
      (elif isFacingUp
        (if (> (LocalVariables|Getz_vel) 0.0)
          (LocalVariables|SetAnimationState "NewEnumerator6")
          (else
            (LocalVariables|SetAnimationState "NewEnumerator2")))
        (return (Utilities|Select :Index (LocalVariables|GetAnimationState) :NewEnumerator0 0 :NewEnumerator1 0 :NewEnumerator2 0 :NewEnumerator3 0 :NewEnumerator4 0 :NewEnumerator5 0 :NewEnumerator6 0 :NewEnumerator7 0))
        (elif isFacingDown
          (if (> 0.0 (LocalVariables|Getz_vel))
            (LocalVariables|SetAnimationState "NewEnumerator7")
            (return (Utilities|Select :Index (LocalVariables|GetAnimationState) :NewEnumerator0 0 :NewEnumerator1 0 :NewEnumerator2 0 :NewEnumerator3 0 :NewEnumerator4 0 :NewEnumerator5 0 :NewEnumerator6 0 :NewEnumerator7 0))
            (else
              (LocalVariables|SetAnimationState "NewEnumerator3"))))))))

(fn MoveSpace
  (params (CollisionBox :type Box%20Component%20Object%20Reference) (isUpDown :type Boolean) (directionLetter :type String))
  (bind _movementarray (Variables|Default|GetmovementArray))
  (LocalVariables|SetisUpDownLoc isUpDown)
  (LocalVariables|SettheDirectionLetter directionLetter)
  (bind _inverse_direction (CallFunction|GetInverseDirection directionLetter))
  (if (== (Utilities|Array|Length (Variables|Default|GetmovementArray)) 0)
    (LocalVariables|SetspaceDelta 1 :!label _label)
    (elif (Utilities|Enum|Equal(Enum) _inverse_direction (Utilities|Array|Get(acopy) (Variables|Default|GetmovementArray) (- (Utilities|Array|Length (Variables|Default|GetmovementArray)) 1)))
      (LocalVariables|SetspaceDelta -1)
      (else
        (goto _label))))
  (for _array_element (Collision|GetOverlappingActors CollisionBox 0 :!class /Script/Engine.PrimitiveComponent)
    (bind _asspace (Utilities|Casting|CastToSpace _array_element))
    (if (LocalVariables|GetisUpDownLoc)
      (if (Variables|Default|GetcanMoveUpDown)
        (if (or (> (Variables|Default|GetdiceRoll) 0) (and (== (Variables|Default|GetdiceRoll) 0) (== (LocalVariables|GetspaceDelta) -1))) :!label _label_2
          (if (and (== (Variables|Default|GetdiceRoll) 0) (== (LocalVariables|GetspaceDelta) -1))
            (Variables|Default|SetCurrentTurnState "NewEnumerator0")
            (Variables|Default|SethasMoved false))
          (Variables|Default|SetvalidMove true)
          (Variables|Default|SetdiceRoll (- (Variables|Default|GetdiceRoll) (LocalVariables|GetspaceDelta)))
          (if (< (LocalVariables|GetspaceDelta) 0)
            (Utilities|Array|RemoveIndex _movementarray (Utilities|Array|LastIndex _movementarray))
            (else
              (Utilities|Array|Add (Variables|Default|GetmovementArray) (LocalVariables|GettheDirectionLetter))))
          (if (== (Variables|Default|GetdiceRoll) 0)
            (Variables|Default|SetCurrentTurnState "NewEnumerator5")
            (Variables|Default|SethasMoved true))
          (return _asspace)))
      (elif (Variables|Default|GetcanMoveLeftRight)
        (goto _label_2)))))

(fn GetInverseDirection
  (params (Input%20Letter :type String))
  (if (Utilities|Enum|Equal(Enum) Input%20Letter "u")
    (LocalVariables|SetreturnString "d")
    (return (LocalVariables|GetreturnString))
    (elif (Utilities|Enum|Equal(Enum) Input%20Letter "d")
      (LocalVariables|SetreturnString "u")
      (return (LocalVariables|GetreturnString))
      (elif (Utilities|Enum|Equal(Enum) Input%20Letter "l")
        (LocalVariables|SetreturnString "r")
        (return (LocalVariables|GetreturnString))
        (elif (Utilities|Enum|Equal(Enum) Input%20Letter "r")
          (LocalVariables|SetreturnString "l")
          (return (LocalVariables|GetreturnString)))))))

(fn RolltheDice
  (bind _returnvalue (Math|Random|RandomInteger 6))
  (bind _returnvalue_2 (+ _returnvalue 1))
  (LocalVariables|SettempRoll -1)
  (Math|Integer|CompareInt (Variables|Default|GetdiceRoll) 0
    (:>
      (if (Utilities|Enum|Equal(Enum) (Variables|Default|GetCurrentTurnState) "NewEnumerator1")
        (LocalVariables|SettempRoll _returnvalue_2 :!label _label)
        (while (== (LocalVariables|GettempRoll) (Variables|Default|GetdiceRoll))
          (LocalVariables|SettempRoll _returnvalue_2))
        (Variables|Default|SetdiceRoll (LocalVariables|GettempRoll))))
    (:==
      (goto _label))
    (:<
      (goto _label))))

(fn GetOccupiedSpaceType
  (for _array_element (Collision|GetOverlappingActors (Variables|Default|GetCollisionCenter) "/Game/Blueprints/Space.Space_C" :!class /Script/Engine.PrimitiveComponent)
    (bind _asspace (Utilities|Casting|CastToSpace _array_element))
    (LocalVariables|Setreturner (Variables|/Game/Blueprints/Space.Space_C|GetType _asspace)))
  (return (LocalVariables|Getreturner)))

(fn DidMove
  (return (Variables|Default|GetBattleMoves)))

(fn Health
  (return (Variables|Default|GetCurrent%20HP) (Variables|Default|GetMax%20HP)))

(fn PlayerandEnemy
  (return self (Variables|Default|GetCurrentEnemy)))

(fn PlayerState
  (return (Variables|Default|GetCurrentTurnState)))

(fn Stats
  (return (+ (Variables|Default|GetBaseAttack) (Variables|Default|GetBuffAttack)) (+ (Variables|Default|GetBaseDefense) (Variables|Default|GetBuffDefense)) (+ (Variables|Default|GetBase%20Magic%20Attack) (Variables|Default|GetBuffMagicAttack)) (+ (Variables|Default|GetBaseMagicDefense) (Variables|Default|GetBuffMagicDefense)) (Variables|Default|GetBaseSpeed)))