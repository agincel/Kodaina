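; Enemy battle actor that holds HP, combat stats and a current move state, apparently for turn-based fights.
; On BeginPlay it registers as the player character's CurrentEnemy and caches unbuffed stats.
; Physical and magic hit events subtract attack minus scaled Defense or MagicDefense, stopping HP at zero and resetting the move state on survival.
; SetMove changes that state, while getter functions expose move, health and stats.
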(event EventBeginPlay
  ;[1 1 1] Begin Play
  (Variables|Default|SetBattleMoves "NewEnumerator0")
  (bind _asmy_character (Utilities|Casting|CastToMyCharacter (Game|Player|GetPlayerPawn 0)))
  (Variables|/Game/Blueprints/MyCharacter.MyCharacter_C|SetCurrentEnemy _asmy_character self)
  (Variables|Default|SetUnbuffedAttack (Variables|Default|GetAttack))
  (Variables|Default|SetUnbuffedDefense (Variables|Default|GetDefense))
  (Variables|Default|SetUnbuffedMagicAttack (Variables|Default|GetMagic%20Attack))
  (Variables|Default|SetUnbuffedMagicDefense (Variables|Default|GetMagic%20Defense)))

(event EventPhysicalAttackHit
  (params (Enemy%20Attack :type Float%20%28single-precision%29))
  ;[1 1 1] Physical Attack Hit
  (if (<= (- (Variables|Default|GetCurrent%20HP) (- Enemy%20Attack (/ (Variables|Default|GetDefense) 1.75))) 0.0)
    (Variables|Default|SetCurrent%20HP 0.0)
    (else
      (Variables|Default|SetCurrent%20HP (- (Variables|Default|GetCurrent%20HP) (- Enemy%20Attack (/ (Variables|Default|GetDefense) 1.75))))
      (Variables|Default|SetBattleMoves "NewEnumerator0"))))

(event EventMagicAttackHit
  (params (Enemy%20Attack :type Float%20%28single-precision%29))
  ;[1 1 1] Magic Attack Hit
  (if (<= (- (Variables|Default|GetCurrent%20HP) (- Enemy%20Attack (/ (Variables|Default|GetMagic%20Defense) 1.75))) 0.0)
    (Variables|Default|SetCurrent%20HP 0.0)
    (else
      (Variables|Default|SetCurrent%20HP (- (Variables|Default|GetCurrent%20HP) (- Enemy%20Attack (/ (Variables|Default|GetMagic%20Defense) 1.75))))
      (Variables|Default|SetBattleMoves "NewEnumerator0"))))

(event EventSetMove
  (params (ToState :type BattleMoveState%20Enum :default "NewEnumerator4"))
  (Variables|Default|SetBattleMoves ToState))

(fn ConstructionScript)

(fn DidMove
  (return (Variables|Default|GetBattleMoves)))

(fn Health
  (return (Variables|Default|GetCurrent%20HP) (Variables|Default|GetMax%20HP)))

(fn PlayerandEnemy
  (return 0 0))

(fn Stats
  (return (Variables|Default|GetAttack) (Variables|Default|GetDefense) (Variables|Default|GetMagic%20Attack) (Variables|Default|GetMagic%20Defense) (Variables|Default|GetSpeed)))